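; BP_CableRandomImpulse is a demo actor that periodically shakes a LoiicCable cable component with random impulses.
; On BeginPlay it starts a looping timer, with a randomly varied start delay, that calls AddRandomImpulse at a configurable interval.
; Each call applies a random unit vector scaled by ImpulseStrength to the cable particle selected by ImpulseIndexParticle, using the component's AddImpulseAtParticleIndex.
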(event `self.ReceiveBeginPlay`
  (`parent.ReceiveBeginPlay`)
  ; At an intervall, add random impulses.
  ; Take a look at the "AddRandomImpulse"function
  (`KismetSystemLibrary.K2_SetTimer` null "AddRandomImpulse" (`self.timeBetweenImpulses`) true false 1.0 0.5))

(fn `AddRandomImpulse`
  ; Send the impulse
  (`LoiicCableComponent.AddImpulseAtParticleIndex` (`self.LoiicCable`) (`self.ImpulseIndexParticle`) (* (`self.impulseStrength`) (`KismetMathLibrary.RandomUnitVector`)) "EImpulseDefault"))

(fn `UserConstructionScript`
  (`parent.UserConstructionScript`))
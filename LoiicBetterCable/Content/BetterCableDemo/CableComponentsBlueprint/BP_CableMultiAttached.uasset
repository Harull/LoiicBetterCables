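; BP_CableMultiAttached is a cable demo actor that pins multiple particles of its LoiicCable to scene components on referenced actors.
; On BeginPlay it walks the ParticleToAttach map, which pairs particle indices with component references.
; Each reference resolves by matching the component name among the referenced actor's root component descendants.
; The matched component is passed to AttachParticleIndexToSceneComponent without a socket, so that particle follows its transform.
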(event `self.ReceiveBeginPlay`
  (`parent.ReceiveBeginPlay`)
  ; Will use the parameter ParticleToAttach, in order to attach particle to their selected scene component.
  (`self.AttachAllParticlesToSceneComponents`))

(fn `AttachAllParticlesToSceneComponents`
  ; Parcour all particles to attach
  (bind (_keypin _valuepin) (`|MapForEach` (`self.ParticleToAttach`))
    (:`then`
      (bind (_otheractor _componentproperty) (break `ComponentReference` _valuepin))
      ; From the component reference structure, we retrieve the corresponding component in our case
      (`/Engine/EditorBlueprintResources/StandardMacros.IsValid` _otheractor
        (:`Is Valid`
          (for _array_element (`SceneComponent.GetChildrenComponents` (`Actor.RootComponent` _otheractor) true)
            (`/Engine/EditorBlueprintResources/StandardMacros.IsValid` _array_element
              (:`Is Valid`
                (if (== (`KismetSystemLibrary.GetObjectName` _array_element) _componentproperty)
                  ; Simply attach the particle index to the scene component. Meaning the particle of the cable at this index, will be linked to the transform of the scene component referenced. (Optionnal socket for skeletal meshes with socket names)
                  (`LoiicCableComponent.AttachParticleIndexToSceneComponent` (`self.LoiicCable`) _keypin _array_element "None")
                  (break))))))))))

(fn `UserConstructionScript`
  (`parent.UserConstructionScript`))
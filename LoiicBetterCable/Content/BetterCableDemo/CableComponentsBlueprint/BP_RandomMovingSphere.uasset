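; BP_RandomMovingSphere is a Better Cable demo actor whose sphere wanders endlessly between random points.
; BeginPlay picks a target, eases the sphere there with MoveComponentTo over a set time, then loops.
; Targets are the area box's location plus its scaled extent times a random 0–1 value per axis, covering only the positive octant.
; The world target becomes relative by subtracting the root's location, ignoring rotation and scale.
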(event `self.ReceiveBeginPlay`
  (`self.SetRandomTargetLocation` :!label _label)
  (`KismetSystemLibrary.MoveComponentTo` (`self.SphereThatMoves`) (- (`self.TargetWorldLocation`) (`SceneComponent.K2_GetComponentLocation` (`self.DefaultSceneRoot`))) (struct) true true (`self.TimeItTakesToMoveToLocation`))
  (goto _label))

(fn `SetRandomTargetLocation`
  (bind (_returnvalue_x _returnvalue_y _returnvalue_z) (`KismetMathLibrary.BreakVector` (`BoxComponent.GetScaledBoxExtent` (`self.AreaWhereSphereMoves`))))
  (set `self.TargetWorldLocation` (+ (`SceneComponent.K2_GetComponentLocation` (`self.AreaWhereSphereMoves`)) (`KismetMathLibrary.MakeVector` (* _returnvalue_x (`KismetMathLibrary.RandomFloat`)) (* _returnvalue_y (`KismetMathLibrary.RandomFloat`)) (* _returnvalue_z (`KismetMathLibrary.RandomFloat`))))))

(fn `UserConstructionScript`)